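; MapPiece_BP is a level segment that chains into an endless track as the main character moves through it.
; Overlapping Box spawns a random piece from PieceList at the ArrowEnd transform, then destroys this piece after a five-second delay.
; Overlapping Box1 prints a game-over message and reloads the current level after a short delay.
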(event OnComponentBeginOverlap(Box)
  (params (OverlappedComponent :type Primitive%20Component%20Object%20Reference) (OtherActor :type Actor%20Object%20Reference) (OtherComp :type Primitive%20Component%20Object%20Reference) (OtherBodyIndex :type Integer) (bFromSweep :type Boolean) (SweepResult :type Hit%20Result%20Structure%20%28by%20ref%29))
  (bind _piecelist (Variables|Default|GetPieceList))
  (Utilities|Casting|CastToMainCharacter_BP OtherActor)
  ;[1 1 1] spawn and destroy platforms
  (Game|SpawnActorfromClass (Utilities|Array|Get(acopy) _piecelist (Math|Random|RandomIntegerinRange 0 (Utilities|Array|LastIndex _piecelist))) (Transformation|GetWorldTransform (Variables|Default|GetArrowEnd)) "Undefined" 0 0)
  (Utilities|FlowControl|Delay 5.0)
  (Actor|DestroyActor))

(event OnComponentBeginOverlap(Box1)
  (params (OverlappedComponent :type Primitive%20Component%20Object%20Reference) (OtherActor :type Actor%20Object%20Reference) (OtherComp :type Primitive%20Component%20Object%20Reference) (OtherBodyIndex :type Integer) (bFromSweep :type Boolean) (SweepResult :type Hit%20Result%20Structure%20%28by%20ref%29))
  (Utilities|Casting|CastToMainCharacter_BP OtherActor)
  (Development|PrintString "GAME OVER")
  (Utilities|FlowControl|Delay 1.0)
  (bind _returnvalue (Game|GetCurrentLevelName true))
  (Game|OpenLevel(byName) (Utilities|String|StringToName _returnvalue)))

(event EventBeginPlay)

(event Collision|EventActorBeginOverlap
  (params (OtherActor :type Actor%20Object%20Reference)))

(event EventTick
  (params (DeltaSeconds :type Float%20%28single-precision%29)))

(fn ConstructionScript)